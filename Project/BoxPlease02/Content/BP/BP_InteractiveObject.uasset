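; BP_InteractiveObject is a physics object that can be carried in front of the player's camera and launched.
; While ObjectPickUp is set, Tick holds it ahead of the main character's camera with physics simulation off, restoring physics on release.
; StartImpuls re-enables physics and applies a strong camera-forward impulse, with DoOnce nodes gating these transitions.
; The Interact event is empty, and neither ObjectPickUp nor StartImpuls is set true here.
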(event EventTick
  (params (DeltaSeconds :type Float%20%28single-precision%29))
  (bind _boxphysics (Variables|Default|GetboxPhysics))
  (Utilities|FlowControl|Sequence
    (:then_0
      (if (not (Variables|Default|GetstartImpuls))
        (if (Variables|Default|GetobjectPickUp)
          (Transformation|SetActorLocation (+ (Transformation|GetWorldLocation (Variables|/Game/BP/BP_MainCharacterController.BP_MainCharacterController_C|GetMainCamera (stale EventBeginPlay _asbp_main_character_controller))) (* (Math|Vector|GetForwardVector (Variables|/Game/BP/BP_MainCharacterController.BP_MainCharacterController_C|GetMainCamera (stale EventBeginPlay _asbp_main_character_controller))) 6e+01)) false false)
          (Utilities|FlowControl|DoOnce false :!label _label
            (:Completed
              (Physics|SetSimulatePhysics _boxphysics false)
              (goto _label_2 Reset)))
          (else
            (Utilities|FlowControl|DoOnce true :!label _label_2
              (:Completed
                (Physics|SetSimulatePhysics _boxphysics true)
                (goto _label Reset)))))))
    (:then_1
      (if (Variables|Default|GetstartImpuls)
        (Utilities|FlowControl|DoOnce false :!label _label_3
          (:Completed
            (Physics|SetSimulatePhysics _boxphysics true)
            (Physics|AddImpulse (Variables|Default|GetboxPhysics) (* (Math|Vector|GetForwardVector (Variables|/Game/BP/BP_MainCharacterController.BP_MainCharacterController_C|GetMainCamera (stale EventBeginPlay _asbp_main_character_controller))) 9e+04) "None" false)
            (Development|PrintString "impuls")
            (Variables|Default|SetstartImpuls false)))
        (else
          (goto _label_3 Reset))))))

(event EventInteract)

(event EventBeginPlay
  (bind _asbp_main_character_controller (Utilities|Casting|CastToBP_MainCharacterController (Game|Player|GetPlayerPawn 0))))

(fn ConstructionScript)